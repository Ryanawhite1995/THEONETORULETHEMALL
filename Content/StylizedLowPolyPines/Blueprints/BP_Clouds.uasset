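; BP_Clouds scatters cloud billboards around the actor as stylized sky dressing.
; The construction script spawns up to NumberOfClouds material billboards, then clears the Update toggle intended for manual repositioning.
; CloudLocation derives random positions from a bounding box around the root, distance offsets and a height range.
; Each billboard is sized by CloudScale and gets one of four random cloud materials, with no active runtime logic.
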(event EventBeginPlay)

(event EventActorBeginOverlap
  (params (OtherActor :type Actor%20Object%20Reference)))

(event EventTick
  (params (DeltaSeconds :type Float%20%28single-precision%29)))

(fn ConstructionScript
  ;[1 1 1] Manual Update to reposition clouds
  (if (Variables|Default|GetUpdate)
    _
    (else
      _))
  ;[1 1 1] Loops for number of clouds input
  (bind _index (Utilities|FlowControl|ForLoopwithBreak 0 (Variables|Default|GetNumber%20of%20Clouds) :!label _label)
    (:LoopBody
      ;[1 1 1] If number of clouds spawned is equal to those requested, stop updating
      (if (not (== _index (Variables|Default|GetNumber%20of%20Clouds)))
        (CallFunction|SpawnClouds)
        (else
          (goto _label Break))))
    (:Completed
      (Variables|Default|SetUpdate false))))

(fn SpawnClouds
  (bind _cloud_scale (Variables|Default|GetCloud%20Scale))
  ;[1 1 1] Adds a cloud billboard to the level
  (bind _returnvalue (AddComponent|AddMaterialBillboardComponent false (Math|Transform|MakeTransform (Utilities|CloudLocation) "0, 0, 0" "500.000000,500.000000,500.000000")))
  (bind _output_get (Variables|Default|SetBillboard _returnvalue))
  (Class|MaterialBillboardComponent|AddElement _returnvalue 0 0 false _cloud_scale _cloud_scale)
  ;[1 1 1] Randomly assigns a material to the billboard based on a random int
  (switch int (Math|Random|RandomIntegerinRange 0 3)
    (:0
      (Rendering|Material|SetMaterial (Variables|Default|GetBillboard) 0 "/Game/StylizedLowPolyPines/Materials/Clouds/Mat_Cloud01.Mat_Cloud01"))
    (:1
      (Rendering|Material|SetMaterial (Variables|Default|GetBillboard) 0 "/Game/StylizedLowPolyPines/Materials/Clouds/Mat_Cloud02.Mat_Cloud02"))
    (:2
      (Rendering|Material|SetMaterial (Variables|Default|GetBillboard) 0 "/Game/StylizedLowPolyPines/Materials/Clouds/Mat_Cloud03.Mat_Cloud03"))
    (:3
      (Rendering|Material|SetMaterial (Variables|Default|GetBillboard) 0 "/Game/StylizedLowPolyPines/Materials/Clouds/Mat_Cloud04.Mat_Cloud04"))))