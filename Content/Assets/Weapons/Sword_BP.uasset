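; Sword Blueprint for a weapon that attaches to the player's ThirdPersonCharacter on pickup.
; Its PickUp event prints a debug string and, if a weapon is already equipped, runs a detach and reposition at the scene root's world transform.
; It then records itself as the character's EquippedWeapon and snaps to the short_weapon_back socket on the character mesh.
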(event EventPickUp
  (bind _returnvalue (Game|GetPlayerCharacter 0))
  (bind _defaultsceneroot (Variables|Default|GetDefaultSceneRoot))
  (bind _asthird_person_character (Utilities|Casting|CastToThirdPersonCharacter _returnvalue))
  (Development|PrintString "Hello")
  (Utilities|IsValid (Variables|/Game/ThirdPersonBP/Blueprints/ThirdPersonCharacter.ThirdPersonCharacter_C|GetEquippedWeapon (.AsThird%20Person%20Character (Utilities|Casting|CastToThirdPersonCharacter (Game|GetPlayerCharacter 0))))
    (:Is%20Valid
      (Transformation|DetachFromActor "KeepRelative" "KeepRelative" "KeepRelative")
      (Transformation|SetActorLocationAndRotation (Transformation|GetWorldLocation _defaultsceneroot) (Transformation|GetWorldRotation _defaultsceneroot)))
    (:Is%20Not%20Valid
      _))
  (Variables|/Game/ThirdPersonBP/Blueprints/ThirdPersonCharacter.ThirdPersonCharacter_C|SetEquippedWeapon _asthird_person_character self)
  (Transformation|AttachComponentToComponent (Variables|/Script/Engine.Character|GetMesh _asthird_person_character) "short_weapon_back" "SnapToTarget" "SnapToTarget" "KeepRelative" true))

(fn ConstructionScript)